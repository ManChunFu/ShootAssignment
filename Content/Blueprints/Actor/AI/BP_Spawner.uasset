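; BP_Spawner is an actor that spawns AI pawns at the position and facing of its Arrow component.
; Its Spawn event takes a SpawnData struct and uses its class, count and behavior tree when that class is valid, otherwise the spawner's own defaults.
; It calls SpawnAIFromClass once per requested pawn in a single loop, all at the same transform.
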(event `/Game/Blueprints/Actor/AI/BPI_Spawnable.Spawn`
  (params (SpawnData :type "/Game/Blueprints/Actor/AI/FSpawnData Structure"))
  (bind (_class _behaviortree _numtospawn) (break `/Game/Blueprints/Actor/AI/FSpawnData` SpawnData))
  (bind _arrow (`self.Arrow`))
  (bind _returnvalue (`KismetSystemLibrary.IsValidClass` _class))
  (for _ (range (select `bool` _returnvalue :`false` (`self.NumToSpawn`) :`true` _numtospawn))
    (`AIBlueprintHelperLibrary.SpawnAIFromClass` (select `bool` _returnvalue :`false` (`self.SpawnClass`) :`true` _class) (select `bool` _returnvalue :`false` (`self.SpawnBehaviorTree`) :`true` _behaviortree) (`SceneComponent.K2_GetComponentLocation` _arrow) (`SceneComponent.K2_GetComponentRotation` _arrow))))

(fn `UserConstructionScript`)