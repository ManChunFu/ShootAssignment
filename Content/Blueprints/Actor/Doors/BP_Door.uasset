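; BP_Door is a door actor that swings open when the player enters its trigger and closes when they leave.
; Trigger overlaps play or reverse the DoorRotation timeline, whose DoorOpen track sets the door's relative yaw.
; Entering and leaving also enable and disable the actor's input for player controller 0, though no input events appear here.
; Tick keeps DoorClose true while the timeline value is below 1.
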(event `self.Trigger.OnComponentBeginOverlap`
  (params (OverlappedComponent :type "PrimitiveComponent Object Reference") (OtherActor :type "Actor Object Reference") (OtherComp :type "PrimitiveComponent Object Reference") (OtherBodyIndex :type Integer) (bFromSweep :type Boolean) (SweepResult :type "HitResult Structure (by ref)"))
  (`/Game/Blueprints/Libraries/BP_MacroLibrary.IsPlayer` OtherActor
    (:`IsPlayer`
      (`self.EnableInput` (`GameplayStatics.GetPlayerController` 0))
      (bind (_direction _dooropen) (`Timeline|DoorRotation` :!label _label)
        (:`Update`
          (`SceneComponent.K2_SetRelativeRotation` (`self.Door`) (`KismetMathLibrary.MakeRotator` 0.0 0.0 _dooropen) false false))))))

(event `self.Trigger.OnComponentEndOverlap`
  (params (OverlappedComponent :type "PrimitiveComponent Object Reference") (OtherActor :type "Actor Object Reference") (OtherComp :type "PrimitiveComponent Object Reference") (OtherBodyIndex :type Integer))
  (`/Game/Blueprints/Libraries/BP_MacroLibrary.IsPlayer` OtherActor
    (:`IsPlayer`
      (`self.DisableInput` (`GameplayStatics.GetPlayerController` 0))
      (goto _label :!via `Reverse`))))

(event `self.ReceiveTick`
  (params (DeltaSeconds :type "Float (single-precision)"))
  (set `self.DoorClose` (< (stale `self.Trigger.OnComponentBeginOverlap` _dooropen) 1.0)))

(fn `UserConstructionScript`)