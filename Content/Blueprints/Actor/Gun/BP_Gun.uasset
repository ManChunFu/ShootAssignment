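; BP_Gun is a gun actor that repeatedly fires BP_Projectile with an animated barrel.
; Shoot waits for GunFireRate, spawns a scaled projectile at ProjectileSpawnPoint, then plays GunFireTimeline to slide the barrel along its local Y axis.
; The timeline's Gun Fired event loops back to the delay while IsTrigger is true, so each cycle, including the first shot, starts with the fire-rate wait.
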(event `Shoot`
  ;[1 1 1] Gun shoots projectile with animation(gun barrel animation while shooting)
  (`KismetSystemLibrary.Delay` (`self.Gun Fire Rate`) :!label _label)
  (`self.Spawn Projectile`)
  (bind (_direction _gun_barrel_location) (`Timeline|Gun Fire Timeline` :!via `PlayFromStart`)
    (:`Update`
      (`self.Move Gun Barrel` _gun_barrel_location))
    (:`Gun Fired`
      (if (`self.IsTrigger`)
        (goto _label)))))

(fn `Move Gun Barrel`
  (params (`Gun Barrel Y Location` :type "Float (double-precision)"))
  (`SceneComponent.K2_SetRelativeLocation` (`self.Gun Barrel`) (`KismetMathLibrary.MakeVector` 0.0 `Gun Barrel Y Location`) false false))

(fn `Spawn Projectile`
  (bind _projectile_spawn_point (`self.Projectile Spawn Point`))
  (`|SpawnActorFromClass` "/Game/Blueprints/Actor/Projectile/BP_Projectile.BP_Projectile_C" (`KismetMathLibrary.MakeTransform` (`SceneComponent.K2_GetComponentLocation` _projectile_spawn_point) (`SceneComponent.K2_GetComponentRotation` _projectile_spawn_point) (`KismetMathLibrary.Conv_DoubleToVector` (`self.Projectile Scale`))) "Undefined" "OverrideRootScale" null null))

(fn `UserConstructionScript`)