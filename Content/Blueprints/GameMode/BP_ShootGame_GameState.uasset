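; BP_ShootGame_GameState is the shooter's game state Blueprint, providing events that show UI for defeat, victory and the final battle.
; GameOver and WinGame each add their own widget to the viewport, then share a delay that ends in quitting the game.
; FinalBattle shows a temporary announcement widget, hiding it after a short delay rather than removing it.
; Each widget receives a reference to this game state when created.
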(event `GameOver`
  (bind _returnvalue (`|CreateWidget` "/Game/UI/WBP_GameOver.WBP_GameOver_C" null self))
  (`UserWidget.AddToViewport` _returnvalue 0)
  (`KismetSystemLibrary.Delay` 5.0 :!label _label)
  (`KismetSystemLibrary.QuitGame` null "Quit"))

(event `WinGame`
  (bind _returnvalue (`|CreateWidget` "/Game/UI/WBP_Win.WBP_Win_C" null self))
  (`UserWidget.AddToViewport` _returnvalue 0)
  (goto _label))

(event `FinalBattle`
  (bind _returnvalue (`|CreateWidget` "/Game/UI/WBP_FinalBattle.WBP_FinalBattle_C" null self))
  (`UserWidget.AddToViewport` _returnvalue 0)
  (`KismetSystemLibrary.Delay` 2.0)
  (`Widget.SetVisibility` _returnvalue "Hidden"))

(fn `UserConstructionScript`)